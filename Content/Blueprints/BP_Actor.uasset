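; BP_Actor is a damageable target that moves between spline points and awards score to the player who damages it.
; Move stores a spline and point count, then starts a looping timer that Cancle clears.
; Each timer tick picks a random point and lerps the actor there with a timeline.
; AnyDamage increments the instigator's MyPlayerState score, twice if the actor has the "Special" tag.
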(event `Cancle`
  (`KismetSystemLibrary.K2_ClearAndInvalidateTimerHandle` (`self.Handle`)))

(event `Move`
  (params (size :type Integer) (Spline :type "SplineComponent Object Reference"))
  (set `self.size` size)
  (set `self.Spline` Spline)
  (bind _returnvalue (`KismetSystemLibrary.K2_SetTimerDelegate` (delegate `MoveBy`) 2.0 true))
  (set `self.Handle` _returnvalue))

(event `MoveBy`
  ;[1 1 1] 位移
  (set `self.Location` (`self.K2_GetActorLocation`))
  (set `self.index` (`KismetMathLibrary.RandomIntegerInRange` 0 (- (`self.size`) 1)))
  (bind (_direction `_新建轨道_0`) (`Timeline|时间轴_0` :!via `PlayFromStart`)
    (:`Update`
      (`self.K2_SetActorLocation` (`KismetMathLibrary.VLerp` (`self.Location`) (`SplineComponent.GetLocationAtSplinePoint` (`self.Spline`) (`self.index`) "World") `_新建轨道_0`)))))

(event `self.ReceiveAnyDamage`
  (params (Damage :type "Float (single-precision)") (DamageType :type "DamageType Object Reference") (InstigatedBy :type "Controller Object Reference") (DamageCauser :type "Actor Object Reference"))
  ;[1 1 1] 击中加分
  (bind _asmy_player_state (cast `/Game/Blueprints/MyPlayerState` (`Controller.PlayerState` InstigatedBy)))
  (if (`self.ActorHasTag` self "Special")
    (`/Game/Blueprints/MyPlayerState.IncrementScore` _asmy_player_state)
    (`/Game/Blueprints/MyPlayerState.IncrementScore` _asmy_player_state)
    (else
      (`/Game/Blueprints/MyPlayerState.IncrementScore` _asmy_player_state))))

(fn `UserConstructionScript`)