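; Spawner actor that creates BP_Actor instances (barrels, per its comment) at random points along the first BP_Spline found in the level.
; BeginPlay caches the spline and its point count, spawns once immediately, then respawns on a looping timer.
; Each new actor receives the spline and size through its Move call.
; A Cancle event stops the timer and calls Cancle on every existing BP_Actor.
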(event `Cancle`
  (`KismetSystemLibrary.K2_ClearAndInvalidateTimerHandle` (`self.Handle`))
  (bind _outactors (`GameplayStatics.GetAllActorsOfClass` "/Game/Blueprints/BP_Actor.BP_Actor_C"))
  (for _array_element _outactors
    (`/Game/Blueprints/BP_Actor.Cancle` _array_element)))

(event `self.ReceiveBeginPlay`
  (bind _returnvalue (`KismetSystemLibrary.K2_SetTimerDelegate` (delegate `Spawn`) 5.0 true))
  (set `self.Handle` _returnvalue)
  (bind _outactors (`GameplayStatics.GetAllActorsOfClass` "/Game/Blueprints/BP_Spline.BP_Spline_C"))
  (bind _spline (`/Game/Blueprints/BP_Spline.Spline` (`|GetArrayItem` _outactors)))
  (set `self.Spline` _spline)
  (set `self.size` (`SplineComponent.GetNumberOfSplinePoints` _spline))
  (`self.Spawn`))

(event `Spawn`
  ;[1 1 1] 生成桶子
  (bind _returnvalue (`|SpawnActorFromClass` "/Game/Blueprints/BP_Actor.BP_Actor_C" (`KismetMathLibrary.MakeTransform` (`SplineComponent.GetLocationAtSplinePoint` (`self.Spline`) (`KismetMathLibrary.RandomIntegerInRange` 0 (- (`self.size`) 1)) "World")) "Undefined" "OverrideRootScale" null null))
  (`/Game/Blueprints/BP_Actor.Move` _returnvalue (`self.size`) (`self.Spline`)))

(fn `UserConstructionScript`)